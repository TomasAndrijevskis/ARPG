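; Boss character Blueprint that reacts to sighted pawns and supports target lock-on.
; PawnSensing passes each seen pawn and the player pawn to DetectPawn, then a DoOnce creates the health widget on the first sighting.
; OnSelect and OnDeselect show and hide the lock-on widget.
; A node to run the BT_Boss behavior tree is present but unconnected, so it never executes here.
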(event `self.ReceiveBeginPlay`)

(event `self.PawnSensing.OnSeePawn`
  (params (Pawn :type "Pawn Object Reference"))
  (`self.DetectPawn` Pawn (`GameplayStatics.GetPlayerPawn` 0))
  (`/Engine/EditorBlueprintResources/StandardMacros.DoOnce` false
    (:`Completed`
      (`self.CreateHealthWidget`))))

(event `self.OnSelect`
  (`SceneComponent.SetVisibility` (`self.Lockon_Widget`) true false))

(event `self.OnDeselect`
  (`SceneComponent.SetVisibility` (`self.Lockon_Widget`) false false))

(fn `UserConstructionScript`)